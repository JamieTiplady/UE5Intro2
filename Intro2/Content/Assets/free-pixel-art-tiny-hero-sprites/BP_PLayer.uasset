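; BP_PLayer is the player character, an Owlet pixel-art sprite that moves left and right and jumps.
; Jump input drives the built-in jump and stop, axis input adds movement along X, and BeginPlay sets the jump velocity.
; Each Tick picks a jump, running or idle flipbook from the movement velocity and flips the sprite's X scale to face the direction of travel.
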(event `self.ReceiveTick`
  (params (DeltaSeconds :type "Float (single-precision)"))
  (bind _sprite (`self.Sprite`))
  (bind (_velocity_x _velocity_y _velocity_z) (`KismetMathLibrary.BreakVector` (`MovementComponent.Velocity` (`self.CharacterMovement`))))
  (bind _returnvalue (>= _velocity_x 0.0))
  (bind _returnvalue_2 (> (`KismetMathLibrary.Abs` _velocity_z) 0.0))
  (if _returnvalue_2
    (`PaperFlipbookComponent.SetFlipbook` _sprite (select `bool` _returnvalue_2 :`false` "/Game/Assets/free-pixel-art-tiny-hero-sprites/2_Owlet_Monster/Owlet_Idle.Owlet_Idle" :`true` "/Game/Assets/free-pixel-art-tiny-hero-sprites/2_Owlet_Monster/Owlet_Jump.Owlet_Jump" :!type "PaperFlipbook Object Reference"))
    (else
      (if true
        _
        (else
          _))
      (`PaperFlipbookComponent.SetFlipbook` _sprite (select `bool` (> (`KismetMathLibrary.Abs` _velocity_x) 0.0) :`false` "/Game/Assets/free-pixel-art-tiny-hero-sprites/2_Owlet_Monster/Owlet_Idle.Owlet_Idle" :`true` "/Game/Assets/free-pixel-art-tiny-hero-sprites/2_Owlet_Monster/Owlet_Running.Owlet_Running" :!type "PaperFlipbook Object Reference"))))
  (if _returnvalue
    _
    (else
      _))
  (`SceneComponent.SetWorldScale3D` (`self.Sprite`) (`KismetMathLibrary.MakeVector` (select `bool` _returnvalue :`false` -1.0 :`true` 1.0) 1.0 1.0)))

(event `self.ReceiveBeginPlay`
  (set `CharacterMovementComponent.JumpZVelocity` 250.0 (`self.CharacterMovement`)))

(event `InputAction|AM_Jump`
  (params (Key :type "Key Structure"))
  (:`Pressed`
    (`self.Jump`))
  (:`Released`
    (`self.StopJumping`)))

(event `InputAxis|AM_MoveLeftRight`
  (params (AxisValue :type "Float (single-precision)"))
  (`self.AddMovementInput` (0.3 0.0 0.0) AxisValue))

(fn `UserConstructionScript`)